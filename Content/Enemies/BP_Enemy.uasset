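; Enemy character that reacts to damage and dies, with a name-derived number label and damage text widgets.
; Damage lowers StatusComponent health, then StateComponent enters hit or dead mode with a matching montage.
; Surviving enemies turn toward the attacker; melee hits also knock them back and briefly flash the outline red via dynamic materials on a master-posed second mesh.
; Death disables capsule collision, and EndDead destroys the actor.
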(event `self.ReceiveBeginPlay`
  (`|ExecutionSequence`
    (:`then_0`
      (for (_array_element _array_index) (`self.Materials`)
        (bind _returnvalue (`KismetMaterialLibrary.CreateDynamicMaterialInstance` _array_element))
        (`PrimitiveComponent.SetMaterial` (`self.CharacterMesh1`) _array_index _returnvalue)
        (`self.ChangeColor` (`self.Color`))))
    (:`then_1`
      (bind _aswb_label (cast `/Game/Widgets/WB_Label` (`WidgetComponent.GetUserWidgetObject` (`self.Label`))))
      (`/Game/Widgets/WB_Label.Update Character` _aswb_label (`KismetStringLibrary.Conv_StringToInt` (`KismetStringLibrary.Replace` (`KismetSystemLibrary.GetObjectName` self) "BP_Enemy"))))))

(event `Combat Text`
  (params (Damage :type "Float (double-precision)"))
  (`/Game/Widgets/WB_Damage.PlayCombatText` (cast `/Game/Widgets/WB_Damage` (`WidgetComponent.GetUserWidgetObject` (`self.DamageWidget`)) :!pure true) Damage))

(event `self.ReceiveAnyDamage`
  (params (Damage :type "Float (single-precision)") (DamageType :type "DamageType Object Reference") (InstigatedBy :type "Controller Object Reference") (DamageCauser :type "Actor Object Reference"))
  (bind _statuscomponent (`self.StatusComponent`))
  (bind _statecomponent (`self.StateComponent`))
  (bind (_returnvalue_roll _returnvalue_pitch _returnvalue_yaw) (`KismetMathLibrary.BreakRotator` (`KismetMathLibrary.FindLookAtRotation` (`self.K2_GetActorLocation`) (`self.K2_GetActorLocation` (`self.Attacker`)))))
  (`|ExecutionSequence`
    (:`then_1`
      (`self.Combat Text` Damage))
    (:`then_2`
      (set `self.Causer` DamageCauser)
      (bind _ascharacter (cast `Character` (`Controller.K2_GetPawn` InstigatedBy)))
      (set `self.Attacker` _ascharacter)
      (bind _output_get (set `self.Damage` Damage))
      (`/Game/Components/StatusComponent.DecreaseHealth` _statuscomponent _output_get)
      (if (<= (`/Game/Components/StatusComponent.Health` _statuscomponent) 0.0)
        (if (not (`/Game/Components/StateComponent.IsDeadMode` _statecomponent))
          (`/Game/Components/StateComponent.SetDeadMode` (`self.StateComponent`))
          (`PrimitiveComponent.SetCollisionEnabled` (`self.CapsuleComponent`) "NoCollision")
          (`self.PlayAnimMontage` "/Game/Character/Montages/Common/Enemy_DeadFall_Montage.Enemy_DeadFall_Montage" 1.0 "Start"))
        (else
          (`/Game/Components/StateComponent.SetHittedMode` _statecomponent)
          (`self.PlayAnimMontage` "/Game/Character/Montages/Common/Enemy_HitReaction_Montage.Enemy_HitReaction_Montage" 1.5)
          (`self.K2_SetActorRotation` (`KismetMathLibrary.MakeRotator` 0.0 0.0 _returnvalue_yaw))
          (cast `/Game/Actions/BP_DoAction_Melee` (`self.Causer`))
          (`self.LaunchCharacter` (* (* (* (`self.GetActorForwardVector`) -1.0) (`CharacterMovementComponent.Mass` (`self.CharacterMovement`))) 2.0) true)
          (for _array_element (`MeshComponent.GetMaterials` (`self.CharacterMesh1`))
            (bind _asmaterial_instance_dynamic (cast `MaterialInstanceDynamic` _array_element))
            (`MaterialInstanceDynamic.SetVectorParameterValue` _asmaterial_instance_dynamic "OutlineColor" (struct :`R` 1.0 :`A` 1.0)))
          (`KismetSystemLibrary.RetriggerableDelay` 0.2)
          (`self.ChangeColor` (`self.Color`)))))))

(event `self.ReceiveTick`
  (params (DeltaSeconds :type "Float (single-precision)")))

(event `self.OnLanded`
  (params (Hit :type "HitResult Structure (by ref)"))
  (`KismetSystemLibrary.PrintString` "Landed"))

(event `self.CapsuleComponent.OnComponentHit`
  (params (HitComponent :type "PrimitiveComponent Object Reference") (OtherActor :type "Actor Object Reference") (OtherComp :type "PrimitiveComponent Object Reference") (NormalImpulse :type "Vector Structure") (Hit :type "HitResult Structure (by ref)")))

(fn `ChangeColor`
  (params (InColor :type "LinearColor Structure"))
  (returns (Result :type Boolean))
  (set `self.Color` InColor)
  (for _array_element (`MeshComponent.GetMaterials` (`self.CharacterMesh1`))
    (bind _asmaterial_instance_dynamic (cast `MaterialInstanceDynamic` _array_element))
    (`MaterialInstanceDynamic.SetVectorParameterValue` _asmaterial_instance_dynamic "OutlineColor" (`local.InColor`)))
  (return false))

(fn `End_Backstep`
  (returns (Result :type Boolean))
  (return false))

(fn `End_Dead`
  (returns (Result :type Boolean))
  (`self.K2_DestroyActor`)
  (return false))

(fn `End_Roll`
  (returns (Result :type Boolean))
  (return false))

(fn `GetCharacterProperties`
  (params (CH_Properties :type "/Game/Player/SV_Playerproperty Object Reference"))
  (returns (Properties :type "/Game/Player/SV_Playerproperty Object Reference"))
  (return null))

(fn `UserConstructionScript`
  (`SkinnedMeshComponent.SetLeaderPoseComponent` (`self.CharacterMesh1`) (`self.Mesh`) false))