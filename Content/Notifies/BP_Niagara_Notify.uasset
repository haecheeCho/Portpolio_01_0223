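; BP_Niagara_Notify is an animation notify state that spawns a configurable Niagara effect from an animation, displayed as "NiagaraEffect".
; On notify begin it spawns the system at the mesh's "EffectSocket" location plus FXOffset, combining the socket rotation with FXRotation.
; The effect is placed in world space without attachment, so the offset ignores socket orientation and the file shows no cleanup on notify end.
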(fn `GetNotifyName`
  (returns (ReturnValue :type String))
  (return "NiagaraEffect"))

(fn `Received_NotifyBegin`
  (params (MeshComp :type "SkeletalMeshComponent Object Reference") (Animation :type "AnimSequenceBase Object Reference") (TotalDuration :type "Float (double-precision)"))
  (returns (ReturnValue :type Boolean))
  (`NiagaraFunctionLibrary.SpawnSystemAtLocation` MeshComp (`self.Niagara`) (+ (`SceneComponent.GetSocketLocation` MeshComp "EffectSocket") (`self.FX Offset`)) (`KismetMathLibrary.ComposeRotators` (`SceneComponent.GetSocketRotation` MeshComp "EffectSocket") (`self.FX Rotation`)))
  (return false))